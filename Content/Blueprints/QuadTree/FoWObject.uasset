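; FoWObject is a fog-of-war block actor that covers its area with a cube mesh.
; The construction script adds that cube with the FoWTest material and collision disabled.
; An unconnected reverse-visibility chain traces from four offset Box1 corners toward a target location, destroying the actor on the first matching hit.
; FireReverseVis is currently empty, so that check never runs.
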(event `FireReverseVis`
  (params (Target :type "Actor Object Reference") (TargetLoc :type "Object.Vector Structure")))

(fn `UserConstructionScript`
  (bind _returnvalue (`AddComponent|StaticMeshComponent_4` :`RelativeTransform` (`KismetMathLibrary.MakeTransform` (0.0 0.0 -30.0) (struct) (1.1 1.1 1.4))))
  (`StaticMeshComponent.SetStaticMesh` _returnvalue "/Engine/EditorMeshes/EditorCube.EditorCube")
  (`PrimitiveComponent.SetMaterial` _returnvalue 0 "/Game/Materials/FoWTest.FoWTest")
  (`PrimitiveComponent.SetCollisionEnabled` _returnvalue "NoCollision")
  (set `self.StaticMesh` _returnvalue))